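; BP_Pistol is a pistol weapon Blueprint that handles shooting and reloading, with ammo state delegated to an ammo component.
; Shoot consumes ammo and spawns a Niagara muzzle flash at the muzzle point, while CanShoot forwards the component's check.
; Reload checks the component, plays a reload montage on the given player, and starts a timer that finishes the reload after the reload duration.
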(event Custom|StartReloadEvent
  (if (Default|CanReload (Variables|Default|GetBP_AmmoComponent))
    (Default|StartReload (Variables|Default|GetBP_AmmoComponent))
    (Utilities|Time|SetTimerbyEvent (delegate Custom|FinishReloadEvent) (Variables|Default|GetReloadDuration))))

(event Custom|FinishReloadEvent
  (Default|FinishReload (Variables|Default|GetBP_AmmoComponent)))

(event EventBeginPlay)

(event Collision|EventActorBeginOverlap
  (params (OtherActor :type Actor%20Object%20Reference)))

(event EventTick
  (params (DeltaSeconds :type Float%20%28single-precision%29)))

(fn ConstructionScript)

(fn Reload
  (params (Player :type BP%20My%20Third%20Person%20Character%20Object%20Reference))
  (if (Default|CanReload (Variables|Default|GetBP_AmmoComponent))
    (CallFunction|StartReloadEvent)
    (Animation|PlayAnimMontage Player "/Game/Characters/Mannequins/Anims/Pistol/MM_Pistol_Reload_Montage.MM_Pistol_Reload_Montage" 1.0 "None")))

(fn Shoot
  (Default|ConsumeAmmo (Variables|Default|GetBP_AmmoComponent))
  (Niagara|SpawnSystemAttached "/Game/NS_MuzzleFlash.NS_MuzzleFlash" (Variables|Default|GetMuzzlePoint) "None" "0, 0, 0" "0, 0, 0" "SnapToTarget" true))

(fn CanShoot
  (return (Default|CanShoot (Variables|Default|GetBP_AmmoComponent))))