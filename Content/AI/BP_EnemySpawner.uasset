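; Enemy spawner actor that places a BP_Enemy at its own transform when play begins and can respawn one on request.
; Each spawned enemy receives a SpawnerRef back to this spawner, presumably so it can call RespawnEnemy.
; RespawnEnemy waits a fixed delay before spawning, and unlike the initial spawn, it skips spawning if a collision cannot be resolved.
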(event Custom|RespawnEnemy
  (Utilities|FlowControl|Delay 5.0)
  (bind _returnvalue (Game|SpawnActorfromClass "/Game/AI/BP_Enemy.BP_Enemy_C" (Transformation|GetActorTransform) "AdjustIfPossibleButDontSpawnIfColliding" "MultiplyWithRoot" 0 0))
  (bind _asbp_enemy (Utilities|Casting|CastToBP_Enemy _returnvalue))
  (Variables|/Game/AI/BP_Enemy.BP_Enemy_C|SetSpawnerRef _asbp_enemy self))

(event EventBeginPlay
  (bind _returnvalue (Game|SpawnActorfromClass "/Game/AI/BP_Enemy.BP_Enemy_C" (Transformation|GetActorTransform) "AdjustIfPossibleButAlwaysSpawn" "MultiplyWithRoot" 0 0))
  (bind _asbp_enemy (Utilities|Casting|CastToBP_Enemy _returnvalue))
  (Variables|/Game/AI/BP_Enemy.BP_Enemy_C|SetSpawnerRef _asbp_enemy self))

(event Collision|EventActorBeginOverlap
  (params (OtherActor :type Actor%20Object%20Reference)))

(event EventTick
  (params (DeltaSeconds :type Float%20%28single-precision%29)))

(fn ConstructionScript)